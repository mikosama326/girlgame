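; Behavior tree service that turns the AI's controlled pawn toward the actor stored in the LookAtActor blackboard key.
; Activation and AI tick events share one path that checks the pawn is valid, then computes a look-at rotation to the target.
; RInterpTo eases the pawn toward it at InterpSpeed, applying the full rotation directly to the actor without isolating yaw.
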(event EventReceiveTickAI
  (params (OwnerController :type AI%20Controller%20Object%20Reference) (ControlledPawn :type Pawn%20Object%20Reference) (DeltaSeconds :type Float%20%28single-precision%29))
  (Utilities|IsValid ControlledPawn
    (:Is%20Valid
      (Transformation|SetActorRotation ControlledPawn (Math|Interpolation|RInterpTo (Transformation|GetActorRotation ControlledPawn) (Math|Rotator|FindLookatRotation (Transformation|GetActorLocation ControlledPawn) (Transformation|GetActorLocation (AI|BehaviorTree|GetBlackboardValueasActor (Variables|Default|GetLookAtActor)))) DeltaSeconds (Variables|Default|GetInterpSpeed))))))

(event EventTick
  (params (OwnerActor :type Actor%20Object%20Reference) (DeltaSeconds :type Float%20%28single-precision%29))
  (Utilities|IsValid (stale EventReceiveTickAI ControlledPawn)
    (:Is%20Valid
      (Transformation|SetActorRotation (stale EventReceiveTickAI ControlledPawn) (Math|Interpolation|RInterpTo (Transformation|GetActorRotation (stale EventReceiveTickAI ControlledPawn)) (Math|Rotator|FindLookatRotation (Transformation|GetActorLocation (stale EventReceiveTickAI ControlledPawn)) (Transformation|GetActorLocation (AI|BehaviorTree|GetBlackboardValueasActor (Variables|Default|GetLookAtActor)))) (stale EventReceiveTickAI DeltaSeconds) (Variables|Default|GetInterpSpeed))))))

(event EventReceiveActivation
  (params (OwnerActor :type Actor%20Object%20Reference))
  (Utilities|IsValid (stale EventReceiveTickAI ControlledPawn)
    (:Is%20Valid
      (Transformation|SetActorRotation (stale EventReceiveTickAI ControlledPawn) (Math|Interpolation|RInterpTo (Transformation|GetActorRotation (stale EventReceiveTickAI ControlledPawn)) (Math|Rotator|FindLookatRotation (Transformation|GetActorLocation (stale EventReceiveTickAI ControlledPawn)) (Transformation|GetActorLocation (AI|BehaviorTree|GetBlackboardValueasActor (Variables|Default|GetLookAtActor)))) (stale EventReceiveTickAI DeltaSeconds) (Variables|Default|GetInterpSpeed))))))