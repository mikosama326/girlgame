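; AI enemy pawn with health, patrol, gun and melee combat, driven by an AICon AI controller.
; On BeginPlay it spawns a weapon onto a mesh socket, firing it only with line of sight and player range.
; Damage events report to perception, then play a hit montage and notify the controller, or ragdoll, unpossess and destroy after a delay.
; A melee sphere overlap starts attack montages whose notifies damage the player.
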(event OnComponentEndOverlap(MeleeSphere)
  (params (OverlappedComponent :type Primitive%20Component%20Object%20Reference) (OtherActor :type Actor%20Object%20Reference) (OtherComp :type Primitive%20Component%20Object%20Reference) (OtherBodyIndex :type Integer))
  ;[1 1 1] End Melee Attack
  (if (== OtherActor (Game|Player|GetPlayerPawn (Class|GameplayStatics|GetPlayerControllerID)))
    (CallFunction|Fire)))

(event OnComponentBeginOverlap(MeleeSphere)
  (params (OverlappedComponent :type Primitive%20Component%20Object%20Reference) (OtherActor :type Actor%20Object%20Reference) (OtherComp :type Primitive%20Component%20Object%20Reference) (OtherBodyIndex :type Integer) (bFromSweep :type Boolean) (SweepResult :type Hit%20Result%20Structure%20%28by%20ref%29))
  ;[1 1 1] Begin Melee Attack
  (if (== OtherActor (Game|Player|GetPlayerPawn (Class|GameplayStatics|GetPlayerControllerID)))
    (CallFunction|MeleeAttack)))

(event Custom|Aiming
  ;[1 1 1] Set state based on aiming
  (Variables|Default|SetbAiming true))

(event Custom|UnAim
  ;[1 1 1] Set state based on aiming
  (Variables|Default|SetbAiming false))

(event Custom|Fire
  (params (TargetObject :type Actor%20Object%20Reference))
  (bind _currentweapon (Variables|Default|GetCurrentWeapon))
  ;[1 1 1] Fire Gun
  (if (Math|Boolean|ANDBoolean (Controller|LineOfSightTo (AI|GetAIController self) TargetObject (+ (Transformation|GetActorLocation) "0, 0,40.000000") false) (<= (Transformation|GetDistanceTo (Game|Player|GetPlayerPawn 0)) (Variables|Default|GetMaxFiringRange)) (not (Variables|Default|GetAmDead)))
    (Default|TriggerPulled _currentweapon)
    (Default|FireCurrentWeapon _currentweapon TargetObject)
    (else
      (Default|TriggerReleased _currentweapon)
      (Default|FireCurrentWeapon _currentweapon TargetObject))))

(event Custom|MeleeAttack
  (bind _attackmontages (Variables|Default|GetAttackMontages))
  (bind _returnvalue (Utilities|Array|Length _attackmontages))
  (bind _returnvalue_2 (- _returnvalue 1))
  (bind _returnvalue_3 (Math|Random|RandomInteger _returnvalue_2))
  (bind _output (Utilities|Array|Get(acopy) _attackmontages _returnvalue_3))
  ;[1 1 1] Melee Animation - WIP
  (if (not (Animation|Montage|MontageIsPlaying (Components|SkeletalMesh|GetAnimInstance (Variables|Character|GetMesh)) _output))
    (Animation|Montage|PlayMontage (Variables|Character|GetMesh) _output
      (:OnNotifyBegin
        (CallFunction|ApplyMeleeDamage)))))

(event Custom|ApplyMeleeDamage
  ;[1 1 1] Melee Damage
  (for _array_element (Collision|GetOverlappingActors (Variables|Default|GetMeleeSphere) "/Script/Engine.Character" :!class /Script/Engine.PrimitiveComponent)
    (if (== _array_element (Game|Player|GetPlayerPawn 0))
      (Game|Damage|ApplyDamage _array_element (Variables|Default|GetMeleeDamage) 0 0))))

(event Custom|PatrolPointMove
  ;[1 1 1] Patrol Logic
  (Variables|Default|SetCurrentPoint (Utilities|Array|Get(acopy) (Variables|Default|GetPatrolPoint) (Variables|Default|GetPatrolIndex)))
  (if (> (Variables|Default|GetPatrolIndex) (- (Utilities|Array|Length (Variables|Default|GetPatrolPoint)) 1))
    (Variables|Default|SetPatrolIndex 0)
    (else
      (bind _result (Math|Integer|IncrementInt (Variables|Default|GetPatrolIndex))
        (:%20%20
          (Variables|Default|SetPatrolIndex _result))))))

(event Custom|PlayDeath
  (bind _currentweapon (Variables|Default|GetCurrentWeapon))
  ;[1 1 1] Damge Events
  (Variables|Default|SetAmDead true)
  (Class|SkeletalMeshComponent|SetAllBodiesSimulatePhysics (Variables|Character|GetMesh) true)
  (Collision|SetCollisionEnabled (Variables|Collision|GetCapsuleComponent) "NoCollision")
  (Utilities|IsValid (Pawn|GetController)
    (:Is%20Valid
      (Pawn|UnPossess (Pawn|GetController)))
    (:Is%20Not%20Valid
      _))
  (Default|TriggerReleased _currentweapon)
  (Default|FireCurrentWeapon _currentweapon)
  (Utilities|FlowControl|RetriggerableDelay (Variables|Default|GetTimeUntilDestroyed))
  (Actor|DestroyActor))

(event Custom|PlayDamage
  (params (StimulusLocation :type Vector))
  (bind _hitmontages (Variables|Default|GetHitMontages))
  (bind _aicon (Variables|Default|GetAICon))
  ;[1 1 1] Damge Events
  (Animation|Montage|PlayMontage (Variables|Character|GetMesh) (Utilities|Array|Get(acopy) _hitmontages (Math|Random|RandomInteger (- (Utilities|Array|Length _hitmontages) 1)))
    (:then
      (Variables|/Game/ActionAISystem/Blueprints/AICon.AICon_C|SetbDamageTaken _aicon true)
      (Variables|/Game/ActionAISystem/Blueprints/AICon.AICon_C|SetStimulusLocation _aicon StimulusLocation)
      (Default|FireOffBTEvents _aicon))))

(event EventBeginPlay
  ;[1 1 1] Create gun in AI hand
  (bind _returnvalue (Game|SpawnActorfromClass (Variables|Default|GetWeaponToSpawn) (Math|Transform|MakeTransform "0, 0, 0") "Undefined" 0 0)) ; Spawn a gun class or it's child
  (bind _asgun (Utilities|Casting|CastToGun _returnvalue))
  (Variables|Default|SetCurrentWeapon _asgun)
  (Transformation|AttachComponentToComponent _returnvalue (Variables|Character|GetMesh) (Variables|Default|GetWeaponSocketName) "KeepRelative" "KeepRelative" "KeepRelative" true) ; Make sure to create a new child class and set it's Socket Name
  (bind _asaicon (Utilities|Casting|CastToAICon (AI|GetAIController self)))
  (Variables|Default|SetAICon _asaicon))

(event Game|Damage|EventPointDamage
  (params (Damage :type Float%20%28single-precision%29) (DamageType :type Damage%20Type%20Object%20Reference) (HitLocation :type Vector :default "0, 0, 0") (HitNormal :type Vector :default "0, 0, 0") (HitComponent :type Primitive%20Component%20Object%20Reference) (BoneName :type Name :default "None") (ShotFromDirection :type Vector :default "0, 0, 0") (InstigatedBy :type Controller%20Object%20Reference) (DamageCauser :type Actor%20Object%20Reference) (HitInfo :type Hit%20Result%20Structure%20%28by%20ref%29))
  ;[1 1 1] Health stuff
  (Class|AISenseDamage|ReportDamageEvent self 0 Damage "0, 0, 0" HitLocation)
  (bind _output_get (Variables|Default|SetfHealth (- (Variables|Default|GetfHealth) Damage)))
  (if (<= _output_get 0.0)
    (CallFunction|PlayDeath)
    (else
      (CallFunction|PlayDamage ShotFromDirection))))

(event EventTick
  (params (DeltaSeconds :type Float%20%28single-precision%29)))

(event Game|Damage|EventAnyDamage
  (params (Damage :type Float%20%28single-precision%29) (DamageType :type Damage%20Type%20Object%20Reference) (InstigatedBy :type Controller%20Object%20Reference) (DamageCauser :type Actor%20Object%20Reference))
  ;[1 1 1] Any Damage
  (Class|AISenseDamage|ReportDamageEvent self 0 Damage "0, 0, 0")
  (bind _output_get (Variables|Default|SetfHealth (- (Variables|Default|GetfHealth) Damage)))
  (if (<= _output_get 0.0)
    (CallFunction|PlayDeath)
    (else
      (CallFunction|PlayDamage "0, 0, 0"))))

(event Game|Damage|EventRadialDamage
  (params (DamageReceived :type Float%20%28single-precision%29) (DamageType :type Damage%20Type%20Object%20Reference) (Origin :type Vector :default "0, 0, 0") (HitInfo :type Hit%20Result%20Structure%20%28by%20ref%29) (InstigatedBy :type Controller%20Object%20Reference) (DamageCauser :type Actor%20Object%20Reference))
  ;[1 1 1] Radial Damge
  (Class|AISenseDamage|ReportDamageEvent self 0 DamageReceived "0, 0, 0" Origin)
  (bind _output_get (Variables|Default|SetfHealth (- (Variables|Default|GetfHealth) DamageReceived)))
  (if (<= _output_get 0.0)
    (CallFunction|PlayDeath)
    (else
      (CallFunction|PlayDamage Origin))))

(fn ConstructionScript)